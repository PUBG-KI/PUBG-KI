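; BP_WaterBodyOcean is an ocean water body that switches the player character in and out of swimming on actor overlap.
; Begin overlap caches the player and the water component's location and bounds height, then starts swimming; end overlap stops it without clearing the reference.
; Tick is debug scaffolding that prints the player mesh location and always "UNDERWATER", since its branch is hardcoded true.
; The cached water values and a disconnected surface-depth query do not feed that check.
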(event `self.ReceiveActorBeginOverlap`
  (params (OtherActor :type "Actor Object Reference"))
  (bind _waterbodycomponent (`self.WaterBodyComponent`))
  (bind _asbp_player_character (cast `/Game/Blueprint/Character/BP_PlayerCharacter` OtherActor))
  (bind _output_get (set `self.As BP Player Character` _asbp_player_character))
  (`/Game/Blueprint/Character/BP_PlayerCharacter.Start Swimming` _output_get)
  (set `self.WaterVolumeLocation` (`SceneComponent.K2_GetComponentLocation` _waterbodycomponent))
  (set `self.WaterVolumeHeight` (.z (`.BoxExtent` (`KismetSystemLibrary.GetComponentBounds` _waterbodycomponent)))))

(event `self.ReceiveActorEndOverlap`
  (params (OtherActor :type "Actor Object Reference"))
  (bind _asbp_player_character (cast `/Game/Blueprint/Character/BP_PlayerCharacter` OtherActor))
  (`/Game/Blueprint/Character/BP_PlayerCharacter.Stop Swimming` _asbp_player_character))

(event `self.ReceiveTick`
  (params (DeltaSeconds :type "Float (single-precision)"))
  (bind _as_bp_player_character (`self.As BP Player Character`)
    (:`then`
      (`KismetSystemLibrary.PrintString` (`KismetStringLibrary.Conv_VectorToString` (`SceneComponent.K2_GetComponentLocation` (`Character.Mesh` _as_bp_player_character))))
      (if true
        (`KismetSystemLibrary.PrintString` "UNDERWATER")
        (else
          (`KismetSystemLibrary.PrintString` "FLOATING"))))
    (:`else`)))

(fn `UserConstructionScript`)