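; BP_TestCharacter is a test character Blueprint whose only live logic toggles the inventory screen.
; Pressing Tab flip-flops InventoryWidget between visible and collapsed, switching between UI and game input modes after a validity check.
; The rest is disconnected scratch nodes for line tracing, look-at interaction, inventory printing, data table lookups and array operations, none of which run.
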(event `Key|Tab`
  (params (Key :type "Key Structure"))
  (bind _inventorywidget (`self.InventoryWidget`))
  (:`Pressed`
    (`/Engine/EditorBlueprintResources/StandardMacros.IsValid` _inventorywidget
      (:`Is Valid`
        (`/Engine/EditorBlueprintResources/StandardMacros.FlipFlop`
          (:`A`
            (`Widget.SetVisibility` _inventorywidget "Visible")
            (`self.InputModeUI`))
          (:`B`
            (`Widget.SetVisibility` _inventorywidget "Collapsed")
            (`self.InputModeGame`)))))))

(event `Key|F`
  (params (Key :type "Key Structure")))

(event `Key|One`
  (params (Key :type "Key Structure")))

(fn `UserConstructionScript`)