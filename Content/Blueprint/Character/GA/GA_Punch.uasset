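; GA_Punch is a Gameplay Ability that plays the player character's punch montages and cannot be canceled once activated.
; While falling, it plays a full-body unarmed power attack montage starting partway in.
; Otherwise, it plays the key 0 entry of its AttackMontage map, unless a prone request or another animation is active, in which case it ends immediately.
; Any montage outcome also ends the ability.
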(event `self.K2_ActivateAbility`
  (bind _returnvalue (`self.GetPlayerCharacterFromActorInfo`))
  (bind _charactermovement (`Character.CharacterMovement` _returnvalue))
  (`self.SetCanBeCanceled` false)
  (if (`NavMovementComponent.IsFalling` _charactermovement)
    (`AbilityTask_PlayMontageAndWait.CreatePlayMontageAndWaitProxy` "None" "/Game/Blueprint/Character/Animation/AnimAssets/Stand/Unarmed/Attack/Unarmed_Combat_Fullbody_PowerAttack_1_Montage.Unarmed_Combat_Fullbody_PowerAttack_1_Montage" 1.0 "None" false 1.0 1.0
      (:`OnCompleted`
        _)
      (:`OnBlendOut`
        _)
      (:`OnInterrupted`
        _)
      (:`OnCancelled`
        _))
    (`self.K2_EndAbility`)
    (elif (and (not (`PlayerMovementComponent.RequestToStartProne` (cast `PlayerMovementComponent` _charactermovement :!pure true))) (not (`PlayerCharacter.bAnimationIsPlaying` _returnvalue)))
      (`AbilityTask_PlayMontageAndWait.CreatePlayMontageAndWaitProxy` "None" (`BlueprintMapLibrary.Map_Find` (`self.AttackMontage`)) 1.0 "None" false
        (:`OnCompleted`
          _)
        (:`OnBlendOut`
          _)
        (:`OnInterrupted`
          _)
        (:`OnCancelled`
          _))
      (`self.K2_EndAbility`)
      (else
        (`self.K2_EndAbility`)))))

(event `self.K2_OnEndAbility`
  (params (bWasCancelled :type Boolean)))