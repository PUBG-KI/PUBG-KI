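; Gameplay ability that makes the player character lean to the right.
; On activation, unless a prone request is set or the character is falling, it plays the right-lean camera movement, starts leaning on the PlayerMovementComponent and adds the InputTag.RightLeaning tag to the actor.
; When the ability ends, it restores the default camera, stops leaning and removes the tag.
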(event `self.K2_ActivateAbility`
  (bind _returnvalue (`self.GetPlayerCharacterFromActorInfo`))
  (bind _asplayer_movement_component (cast `PlayerMovementComponent` (`Character.CharacterMovement` (`self.GetPlayerCharacterFromActorInfo`))))
  (if (and (not (`PlayerMovementComponent.RequestToStartProne` _asplayer_movement_component)) (not (`NavMovementComponent.IsFalling` _asplayer_movement_component)))
    (`PlayerCharacter.RightLeanCameraMovement` _returnvalue)
    (`PlayerMovementComponent.StartLeaning` _asplayer_movement_component 1.0)
    (`BaseFunctionLibrary.AddGameplayTagToActor` _returnvalue (struct :`TagName` "InputTag.RightLeaning"))))

(event `self.K2_OnEndAbility`
  (params (bWasCancelled :type Boolean))
  (bind _returnvalue (`self.GetPlayerCharacterFromActorInfo`))
  (`PlayerCharacter.RightDefaultCameraMovement` _returnvalue)
  (bind _asplayer_movement_component (cast `PlayerMovementComponent` (`Character.CharacterMovement` _returnvalue)))
  (`PlayerMovementComponent.StopLeaning` _asplayer_movement_component)
  (`BaseFunctionLibrary.RemoveGameplayTagFromActor` _returnvalue (struct :`TagName` "InputTag.RightLeaning")))