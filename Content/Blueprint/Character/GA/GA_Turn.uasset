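; GA_Turn is a gameplay ability that plays a 90-degree turn-in-place montage for the unarmed combat player character.
; On activation, the sign of the yaw delta between base aim and actor rotation selects left or right, and prone, crouch or standing state selects the montage.
; It enables Use Controller Desired Rotation during the turn, ends when the montage finishes or is interrupted, and switches that setting off on end.
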(event `self.K2_ActivateAbility`
  (bind (_returnvalue_roll _returnvalue_pitch _returnvalue_yaw) (`KismetMathLibrary.BreakRotator` (`KismetMathLibrary.NormalizedDeltaRotator` (`Pawn.GetBaseAimRotation` (`self.GetPlayerCharacterFromActorInfo`)) (`self.Character Rotation`))))
  (set `self.Character Rotation` (`Actor.K2_GetActorRotation` (`self.GetPlayerCharacterFromActorInfo`)))
  (bind _output_get (set `self.Save Delta Z` _returnvalue_yaw))
  ;[1 1 1] True->Left
  (if (< _output_get 0.0)
    (set `CharacterMovementComponent.bUseControllerDesiredRotation` true (`Character.CharacterMovement` (`self.GetPlayerCharacterFromActorInfo`)))
    (`AbilityTask_PlayMontageAndWait.CreatePlayMontageAndWaitProxy` "None" (select `bool` (`PlayerCharacter.GetIsProne` (`self.GetPlayerCharacterFromActorInfo`)) :`false` (select `bool` (`PlayerCharacter.GetIsCrouch` (`self.GetPlayerCharacterFromActorInfo`)) :`false` "/Game/Blueprint/Character/Animation/AnimAssets/Stand/Unarmed/Unarmed_Combat_Stand_Turn_L_90_Montage.Unarmed_Combat_Stand_Turn_L_90_Montage" :`true` "/Game/Blueprint/Character/Animation/AnimAssets/Crouch/Unarmed/Unarmed_Combat_Crouch_Turn_L_90_Montage.Unarmed_Combat_Crouch_Turn_L_90_Montage" :!type "AnimMontage Object Reference") :`true` "/Game/Blueprint/Character/Animation/AnimAssets/Prone/Unarmed/Unarmed_Combat_Prone_Turn_L_90_Montage.Unarmed_Combat_Prone_Turn_L_90_Montage")
      (:`OnCompleted`
        _)
      (:`OnBlendOut`
        _)
      (:`OnInterrupted`
        _)
      (:`OnCancelled`
        _))
    (`self.K2_EndAbility`)
    (else
      (`AbilityTask_PlayMontageAndWait.CreatePlayMontageAndWaitProxy` "None" (select `bool` (`PlayerCharacter.GetIsProne` (`self.GetPlayerCharacterFromActorInfo`)) :`false` (select `bool` (`PlayerCharacter.GetIsCrouch` (`self.GetPlayerCharacterFromActorInfo`)) :`false` "/Game/Blueprint/Character/Animation/AnimAssets/Stand/Unarmed/Unarmed_Combat_Stand_Turn_R_90_Montage.Unarmed_Combat_Stand_Turn_R_90_Montage" :`true` "/Game/Blueprint/Character/Animation/AnimAssets/Crouch/Unarmed/Unarmed_Combat_Crouch_Turn_R_90_Montage.Unarmed_Combat_Crouch_Turn_R_90_Montage" :!type "AnimMontage Object Reference") :`true` "/Game/Blueprint/Character/Animation/AnimAssets/Prone/Unarmed/Unarmed_Combat_Prone_Turn_R_90_Montage.Unarmed_Combat_Prone_Turn_R_90_Montage")
        (:`then`
          (set `CharacterMovementComponent.bUseControllerDesiredRotation` true (`Character.CharacterMovement` (`self.GetPlayerCharacterFromActorInfo`))))
        (:`OnCompleted`
          (`self.K2_EndAbility` :!label _label))
        (:`OnBlendOut`
          (goto _label))
        (:`OnInterrupted`
          (goto _label))
        (:`OnCancelled`
          (goto _label))))))

(event `self.K2_OnEndAbility`
  (params (bWasCancelled :type Boolean))
  (set `CharacterMovementComponent.bUseControllerDesiredRotation` false (`Character.CharacterMovement` (`self.GetPlayerCharacterFromActorInfo`))))