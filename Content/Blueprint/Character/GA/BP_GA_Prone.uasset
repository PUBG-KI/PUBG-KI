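; Gameplay ability that toggles the player character's prone stance, keyed on the Player.State.Prone tag.
; If the tag is present, it clears the prone flag and tag immediately and ends without playing a montage.
; Otherwise it plays the stand-to-prone montage, setting both on completion or blend out.
; An interrupted or cancelled montage ends the ability without changing state.
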(event `self.K2_ActivateAbility`
  (bind _returnvalue (`self.GetPlayerCharacterFromActorInfo`))
  (`BaseFunctionLibrary.BP_HasTag` (`self.GetPlayerCharacterFromActorInfo`) (struct :`TagName` "Player.State.Prone")
    (:`Yes`
      (`PlayerCharacter.SetIsProne` _returnvalue false)
      (`BaseFunctionLibrary.RemoveGameplayTagFromActor` _returnvalue (struct :`TagName` "Player.State.Prone"))
      (`self.K2_EndAbility`))
    (:`No`
      (`AbilityTask_PlayMontageAndWait.CreatePlayMontageAndWaitProxy` "None" "/Game/Blueprint/Character/Animation/AnimAssets/TransPosture/StandToProneMontage.StandToProneMontage" 1.0 "None" false
        (:`OnCompleted`
          (`PlayerCharacter.SetIsProne` (`self.GetPlayerCharacterFromActorInfo`) true :!label _label)
          (`BaseFunctionLibrary.AddGameplayTagToActor` (`self.GetPlayerCharacterFromActorInfo`) (struct :`TagName` "Player.State.Prone"))
          (`self.K2_EndAbility`))
        (:`OnBlendOut`
          (goto _label))
        (:`OnInterrupted`
          (`self.K2_EndAbility` :!label _label_2))
        (:`OnCancelled`
          (goto _label_2))))))