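; Gameplay ability for AKM weapon fire, spawning projectiles while the current gun has ammo.
; Single mode fires once and ends, while Auto repeats on a looping timer; the three-round burst logic exists but is never started.
; SpawnBullet passes weapon ballistics data to BP_Projectile, spawning it only without authority.
; Ending with an empty magazine activates abilities by tag for automatic reload.
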(event `self.K2_ActivateAbilityFromEvent`
  (params (EventData :type "GameplayEventData Structure (by ref)"))
  ;[1 1 1] Comment
)

(event `Auto_fire`
  ;[1 1 1] 연발
  (if (> (`Gun_Base.GetBulletArmo` (`InventoryComponent.GetCurrentWeapon_GunBase` (`PlayerCharacter.InventoryComponent` (`self.GetPlayerCharacterFromActorInfo`)))) 0.0)
    (`self.SpawnBullet`)))

(event `self.K2_ActivateAbility`
  (if (> (`Gun_Base.GetBulletArmo` (`InventoryComponent.GetCurrentWeapon_GunBase` (`PlayerCharacter.InventoryComponent` (`self.GetPlayerCharacterFromActorInfo`)))) 0.0)
    (switch `EFiremodes` (`Gun_Base.GetFireMode` (`InventoryComponent.GetCurrentWeapon_GunBase` (`PlayerCharacter.InventoryComponent` (`self.GetPlayerCharacterFromActorInfo`))))
      (:`Auto`
        ;[1 1 1] 연발
        (`self.SpawnBullet`
          (:`Success`
            (bind _returnvalue (`KismetSystemLibrary.K2_SetTimerDelegate` (delegate `Auto_fire`) 0.1 true))
            (set `self.AutoHandle` _returnvalue))))
      (:`Single`
        ;[1 1 1] 단발
        (`self.SpawnBullet`
          (:`Success`
            (`self.K2_EndAbility`)))))
    (else
      (`self.K2_EndAbility`)
      (`KismetSystemLibrary.PrintString` "aaaaaaaaaaaaaa"))))

(event `self.K2_OnEndAbility`
  (params (bWasCancelled :type Boolean))
  ;[1 1 1] 자동 재장전
  (if (<= (`Gun_Base.GetBulletArmo` (`InventoryComponent.GetCurrentWeapon_GunBase` (`PlayerCharacter.InventoryComponent` (`self.GetPlayerCharacterFromActorInfo`)))) 0.0)
    (`AbilitySystemComponent.TryActivateAbilitiesByTag` (`self.GetAbilitySystemComponentFromActorInfo`) (`self.Gameplay Tag Container`) true)))

(event `Semi_Auto`
  ;[1 1 1] 3점사
  (bind _counter (`/Engine/EditorBlueprintResources/StandardMacros.Do N` 2 :!label _label)
    (:`Exit`
      (if (> (`Gun_Base.GetBulletArmo` (`InventoryComponent.GetCurrentWeapon_GunBase` (`PlayerCharacter.InventoryComponent` (`self.GetPlayerCharacterFromActorInfo`)))) 0.0)
        (`self.SpawnBullet`
          (:`Success`
            (if (== _counter 2)
              (`KismetSystemLibrary.K2_ClearAndInvalidateTimerHandle` (`self.SemiHandle`))
              (`|ExecutionSequence`
                (:`then_0`
                  (`KismetSystemLibrary.Delay` 0.3)
                  (`self.K2_EndAbility`))
                (:`then_1`
                  (goto _label :!via `Reset`)))
              (else
                (`KismetSystemLibrary.PrintString` "Single")))))
        (else
          (`KismetSystemLibrary.K2_ClearAndInvalidateTimerHandle` (`self.SemiHandle`))
          (goto _label :!via `Reset`))))))