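; Gameplay ability that reloads the player's current gun, ending at once if its ammo is already full.
; It blocks cancellation, runs a zoom check without authority, and picks a montage by prone state and whether the gun is empty.
; Montage gameplay events move the magazine between hand and weapon sockets, toggle its visibility, and refill ammo from the weapon data asset at reload end.
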(event `self.K2_ActivateAbility`
  (bind _reload_charge_true_montage (`self.Reload Charge True Montage`))
  (bind _returnvalue (`EquippedComponent.GetCurrentWeapon_GunBase` (`PlayerCharacter.EquippedComponent` (`self.GetPlayerCharacterFromActorInfo`))))
  (bind _returnvalue_2 (`EquippedComponent.GetCurrentWeapon_GunBase` (`PlayerCharacter.EquippedComponent` (`self.GetPlayerCharacterFromActorInfo`))))
  (bind _returnvalue_3 (`EquippedComponent.GetCurrentWeapon_GunBase` (`PlayerCharacter.EquippedComponent` (`self.GetPlayerCharacterFromActorInfo`))))
  (bind _returnvalue_4 (`Gun_Base.GetBulletArmo` _returnvalue_2))
  (bind _returnvalue_5 (`Gun_Base.GetMagToHandSocekt` (`EquippedComponent.GetCurrentWeapon_GunBase` (`PlayerCharacter.EquippedComponent` (`self.GetPlayerCharacterFromActorInfo`)))))
  (bind _returnvalue_6 (`Gun_Base.GetMagToHandSocekt` (`EquippedComponent.GetCurrentWeapon_GunBase` (`PlayerCharacter.EquippedComponent` (`self.GetPlayerCharacterFromActorInfo`)))))
  (`self.SetCanBeCanceled` false)
  (`|ExecutionSequence`
    (:`then_0`
      (`self.K2_HasAuthority`
        (:`False`
          (`self.CheckZoom`))))
    (:`then_1`
      (if (not (== _returnvalue_4 (`.Armo` (break `WeaponData` (`Weapon_Base.GetWeaponDataAsset` _returnvalue_2)))))
        (bind (_asynctaskproxy _eventtag) (`PlayMontageAndWaitForEvent.PlayMontageAndWaitForEvent` "None" (`self.selectCurrentMontage_isProne_Reload` (`|GetArrayItem` _reload_charge_true_montage) (`|GetArrayItem` _reload_charge_true_montage 1) (`|GetArrayItem` _reload_charge_true_montage 2) (`|GetArrayItem` _reload_charge_true_montage 3) (== _returnvalue_4 0.0)) (struct :`GameplayTags` (struct :`(TagName` "Player.Event.Action.ReloadEnd") :`(TagName` "Player.Event.Action.Reload") :`(TagName` "Player.Event.Action.VisibleMag") :`(TagName` "Player.Event.Action.HideMag"))))
          (:`OnCompleted`
            (`self.K2_EndAbility` :!label _label))
          (:`OnBlendOut`
            (goto _label))
          (:`OnInterrupted`
            (goto _label))
          (:`OnCancelled`
            (goto _label))
          (:`EventReceived`
            (`|SwitchGameplayTag` _eventtag
              (:`Player.Event.Action.Reload`
                (`ActorComponent.SetIsReplicated` _returnvalue_6 true)
                (`SceneComponent.K2_AttachToComponent` _returnvalue_6 (`self.GetOwningComponentFromActorInfo`) "item_lSocket" "SnapToTarget" "SnapToTarget" "KeepRelative" true))
              (:`Player.Event.Action.ReloadEnd`
                (`|ExecutionSequence`
                  (:`then_0`
                    (`SceneComponent.K2_AttachToComponent` (`Gun_Base.GetMagToHandSocekt` _returnvalue_3) (`Weapon_Base.WeaponSkeletalMeshComponent` _returnvalue_3) "MagSocket" "SnapToTarget" "SnapToTarget" "KeepRelative" true))
                  (:`then_1`
                    (`Gun_Base.SetBulletArom` _returnvalue (`.Armo` (break `WeaponData` (`Weapon_Base.GetWeaponDataAsset` _returnvalue))))
                    (`KismetSystemLibrary.PrintString` (`KismetStringLibrary.Conv_DoubleToString` (`Gun_Base.GetBulletArmo` _returnvalue))))))
              (:`Player.Event.Action.HideMag`
                (`SceneComponent.SetVisibility` _returnvalue_5 false false))
              (:`Player.Event.Action.VisibleMag`
                (`SceneComponent.SetVisibility` _returnvalue_5 true false)))))
        (else
          (`self.K2_EndAbility`))))))