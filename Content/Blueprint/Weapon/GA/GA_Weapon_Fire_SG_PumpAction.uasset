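; Pump-action shotgun fire gameplay ability that shoots a spread of pellets when the current gun has ammo.
; SpawnBullet plays the pose-specific recoil montage and, on the non-authority side only, spawns multiple BP_Projectile actors with weapon-data ballistics and randomized velocity offsets.
; A follow-up montage then plays, and the ability ends when it finishes or is interrupted.
; On ending with an empty magazine, it activates abilities by tag to auto-reload.
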(event `self.K2_ActivateAbilityFromEvent`
  (params (EventData :type "GameplayEventData Structure (by ref)"))
  ;[1 1 1] Comment
)

(event `self.K2_ActivateAbility`
  (`self.SetCanBeCanceled` false)
  (if (> (`Gun_Base.GetBulletArmo` (`EquippedComponent.GetCurrentWeapon_GunBase` (`PlayerCharacter.EquippedComponent` (`self.GetPlayerCharacterFromActorInfo`)))) 0.0)
    ;[1 1 1] 단발
    (`self.SpawnBullet`
      (:`Success`
        (`PlayMontageAndWaitForEvent.PlayMontageAndWaitForEvent` "None" (`self.Montage to Play_0`) (struct) 2.0 "Default"
          (:`OnCompleted`
            _)
          (:`OnBlendOut`
            _)
          (:`OnInterrupted`
            _)
          (:`OnCancelled`
            _))
        (`self.K2_EndAbility`)))
    (else
      (`self.K2_EndAbility`))))

(event `self.K2_OnEndAbility`
  (params (bWasCancelled :type Boolean))
  ;[1 1 1] 자동 재장전
  (if (<= (`Gun_Base.GetBulletArmo` (`EquippedComponent.GetCurrentWeapon_GunBase` (`PlayerCharacter.EquippedComponent` (`self.GetPlayerCharacterFromActorInfo`)))) 0.0)
    (`AbilitySystemComponent.TryActivateAbilitiesByTag` (`self.GetAbilitySystemComponentFromActorInfo`) (`self.Gameplay Tag Container`) true)))