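; Gameplay ability that performs the visual weapon reload, playing a fixed AK tactical reload montage on the owning mesh while non-cancelable.
; Gameplay events during the montage attach the current gun's magazine to the character's left-hand item socket, then back to the weapon's mag socket.
; The ability ends when the montage completes; the alternate branch is an unreachable placeholder behind a hardcoded true condition, and no ammo logic is present.
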(event `self.K2_ActivateAbility`
  (bind _returnvalue (`InventoryComponent.GetCurrentWeapon_GunBase` (`PlayerCharacter.InventoryComponent` (`self.GetPlayerCharacterFromActorInfo`))))
  (`self.SetCanBeCanceled` false)
  (if true
    ;[1 1 1] Charge / Tactical Reload animation
    (`|PlayMontage` (`self.GetOwningComponentFromActorInfo`) "/Game/Blueprint/Character/Animation/AnimAssets/Reload/AK/tactical/Weapon_AK_Reload_Tactical_Base_Montage.Weapon_AK_Reload_Tactical_Base_Montage"
      (:`then`
        (`|ExecutionSequence`
          (:`then_0`
            (`AbilityTask_WaitGameplayEvent.WaitGameplayEvent` (struct :`TagName` "Player.Event.Action.Reload") null
              (:`EventReceived`
                (`SceneComponent.K2_AttachToComponent` (`Gun_Base.GetMagToHandSocekt` (`InventoryComponent.GetCurrentWeapon_GunBase` (`PlayerCharacter.InventoryComponent` (`self.GetPlayerCharacterFromActorInfo`)))) (`self.GetOwningComponentFromActorInfo`) "item_lSocket" "SnapToTarget" "SnapToTarget" "KeepRelative" true))))
          (:`then_1`
            (`AbilityTask_WaitGameplayEvent.WaitGameplayEvent` (struct :`TagName` "Player.Event.Action.ReloadEnd") null
              (:`EventReceived`
                (`SceneComponent.K2_AttachToComponent` (`Gun_Base.GetMagToHandSocekt` _returnvalue) (`Weapon_Base.WeaponSkeletalMeshComponent` _returnvalue) "MagSocket" "SnapToTarget" "SnapToTarget" "KeepRelative" true))))))
      (:`OnCompleted`
        (`self.K2_EndAbility`)))
    (else
      (`|PlayMontage` null
        (:`then`
          _)
        (:`OnCompleted`
          _))
      (`self.K2_EndAbility`))))

(event `self.K2_OnEndAbility`
  (params (bWasCancelled :type Boolean)))