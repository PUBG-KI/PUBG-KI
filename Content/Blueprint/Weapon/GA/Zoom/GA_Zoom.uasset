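; GA_Zoom is a Gameplay Ability that toggles weapon zoom by switching the player between the follow camera and the first-person camera.
; On activation it checks the character's IsZoom flag.
; When not zoomed, it calls ActivatedZoom with the current weapon's skeletal mesh and the first-person camera; otherwise DeActivatedZoom restores the follow camera.
; The ability ends immediately after either call.
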(event `self.K2_ActivateAbility`
  (bind _returnvalue (`self.GetPlayerCharacterFromActorInfo`))
  (bind _returnvalue_2 (`self.GetPlayerCharacterFromActorInfo`))
  (if (not (`PlayerCharacter.IsZoom` (`self.GetPlayerCharacterFromActorInfo`)))
    (`self.ActivatedZoom` (`Weapon_Base.WeaponSkeletalMeshComponent` (`EquippedComponent.GetCurrentWeapon` (`PlayerCharacter.EquippedComponent` _returnvalue_2))) (`PlayerCharacter.FirstPersonCamera` _returnvalue_2) (`PlayerCharacter.FollowCamera` _returnvalue_2))
    (`self.K2_EndAbility`)
    (else
      (`self.DeActivatedZoom` (`PlayerCharacter.FollowCamera` _returnvalue) (`PlayerCharacter.FirstPersonCamera` _returnvalue))
      (`self.K2_EndAbility`))))