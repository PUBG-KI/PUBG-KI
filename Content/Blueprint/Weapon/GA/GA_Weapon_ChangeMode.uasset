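; Gameplay ability that toggles the player's current gun between single and automatic fire.
; On activation it proceeds only if the player mesh runs ABP_PlayerCharacter.
; It reads the fire mode of the InventoryComponent's current weapon, switches Single to Auto or any other mode to Single via ChangeFiremodeAR, then ends the ability.
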(event `self.K2_ActivateAbility`
  (bind _returnvalue (`InventoryComponent.GetCurrentWeapon_GunBase` (`PlayerCharacter.InventoryComponent` (`self.GetPlayerCharacterFromActorInfo`))))
  (bind _asabp_player_character (cast `/Game/Blueprint/Character/Animation/ABP_PlayerCharacter` (`SkeletalMeshComponent.GetAnimInstance` (`Character.Mesh` (`self.GetPlayerCharacterFromActorInfo`)))))
  (`/Engine/EditorBlueprintResources/StandardMacros.IsValid` _asabp_player_character
    (:`Is Valid`
      (if (`|EnumEquality` (`Gun_Base.GetFireMode` _returnvalue) "Single")
        (`Gun_Base.ChangeFiremode_AR` _returnvalue "Auto")
        (else
          (`Gun_Base.ChangeFiremode_AR` _returnvalue "Single")))
      (`self.K2_EndAbility`))))