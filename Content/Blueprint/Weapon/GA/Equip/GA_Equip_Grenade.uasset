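; Gameplay ability that switches the player to the grenade in the throwable slot, ending early if that slot is empty or already current.
; Event-driven montages stow the current weapon by type and stance, then play the throwable's montage in reverse to attach it to the hand.
; Equip and unequip handlers swap anim layer, local input mapping context, granted weapon abilities and replicated weapon tag, using each weapon's data.
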(event `SetAnimLayer`
  (params (InClass :type "AnimInstance Class Reference"))
  ;[1 1 1] 코멘트
  (`SkeletalMeshComponent.LinkAnimClassLayers` (`self.GetOwningComponentFromActorInfo`) InClass))

(event `RemoveWeaponAbility`
  (params (Target :type "Weapon_Base Object Reference"))
  ;[1 1 1] 코멘트
  (`BaseAbilitySystemComponent.RemoveGrantedPlayerWeaponAbilities` (`self.GetBaseAbilitySystemComponentFromActorInfo`) (`Weapon_Base.GetGrantedAbilitySpecHandles` Target)))

(event `SetWeaponAbility`
  (params (WeaponAbilities :type "Array of PlayerAbilitySet Structure (by ref)") (Target :type "Weapon_Base Object Reference"))
  ;[1 1 1] 코멘트
  (bind _outgrantedabilityspechandles (`BaseAbilitySystemComponent.GrantPlayerWeaponAbilities` (`self.GetBaseAbilitySystemComponentFromActorInfo`) WeaponAbilities (`self.GetAbilityLevel`)))
  (`Weapon_Base.AssignGrantedAbilitySpecHandles` Target _outgrantedabilityspechandles)
  (`KismetSystemLibrary.PrintString` "Hello"))

(event `self.K2_ActivateAbility`
  (bind _returnvalue (`EquippedComponent.GetThrowableSlot` (`PlayerCharacter.EquippedComponent` (`self.GetPlayerCharacterFromActorInfo`))))
  (bind _returnvalue_2 (`EquippedComponent.GetThrowableSlot` (`PlayerCharacter.EquippedComponent` (`self.GetPlayerCharacterFromActorInfo`))))
  (bind _returnvalue_3 (`KismetSystemLibrary.IsValid` _returnvalue))
  (`KismetSystemLibrary.PrintString` (`KismetStringLibrary.Conv_BoolToString` _returnvalue_3))
  (if _returnvalue_3
    (`self.SetCanBeCanceled` false)
    (if (`self.EqualCurrentWeapon` _returnvalue)
      (`KismetSystemLibrary.PrintString` "No Change Weapon")
      (`self.K2_EndAbility`)
      (else
        (if (`self.IsValidCurrentWeapon`)
          (switch `EGunType` (`.Type` (break `WeaponData` (`Weapon_Base.GetWeaponDataAsset` (`EquippedComponent.GetCurrentWeapon` (`PlayerCharacter.EquippedComponent` (`self.GetPlayerCharacterFromActorInfo`))))))
            (:`AR`
              (`PlayMontageAndWaitForEvent.PlayMontageAndWaitForEvent` "None" (`self.selectCurrentMontage_isProne_PrimarySecondary` "/Game/Blueprint/Character/Animation/AnimAssets/Prone/Rifle/Rifle_Combat_Prone_PrimarySlot_Montage.Rifle_Combat_Prone_PrimarySlot_Montage" "/Game/Blueprint/Character/Animation/AnimAssets/Stand/Equip/Frimary/Rifle_Combat_Stand_PrimarySlot_Static_Montage.Rifle_Combat_Stand_PrimarySlot_Static_Montage" "/Game/Blueprint/Character/Animation/AnimAssets/Prone/Rifle/Rifle_Combat_Prone_SecondarySlot_Montage.Rifle_Combat_Prone_SecondarySlot_Montage" "/Game/Blueprint/Character/Animation/AnimAssets/Stand/Equip/Secondary/Rifle_Combat_Stand_SecondarySlot_Static_Montage.Rifle_Combat_Stand_SecondarySlot_Static_Montage" (`self.EqualCurrentWeaponToPrimaryWeaponSlot`)) (struct :`GameplayTags` (struct :`(TagName` "Player.Event.Action.UnEquip"))) 2.0 "UnEquip" :!label _label
                (:`EventReceived`
                  _)))
            (:`SR`
              (goto _label))
            (:`DMR`
              (goto _label))
            (:`SMG`
              (goto _label))
            (:`SG`
              (goto _label))
            (:`Pistol`
              (`PlayMontageAndWaitForEvent.PlayMontageAndWaitForEvent` "None" (`self.selectCurrentMontage_isProne` "/Game/Blueprint/Character/Animation/AnimAssets/Prone/Rifle/Rifle_Combat_Prone_PistolSlot_Montage.Rifle_Combat_Prone_PistolSlot_Montage" "/Game/Blueprint/Character/Animation/AnimAssets/Stand/Equip/Pistol/AM_Pistol_Equip_UnEquip.AM_Pistol_Equip_UnEquip") (struct :`GameplayTags` (struct :`(TagName` "Player.Event.Action.UnEquip"))) 2.0 "UnEquip"
                (:`EventReceived`
                  (`self.setSocketName` "SideArm")))))
          (`self.UnEquipWeapon`)
          (`KismetSystemLibrary.Delay` 0.05))
        (`PlayMontageAndWaitForEvent.PlayMontageAndWaitForEvent` "None" (`self.selectCurrentMontage_isProne` "/Game/Blueprint/Character/Animation/AnimAssets/Stand/Equip/Thorwable/Equip_throwable_F_BaseBody_01_Rifle_Combat_Prone_Throw_Unequip_Montage.Equip_throwable_F_BaseBody_01_Rifle_Combat_Prone_Throw_Unequip_Montage" "/Game/Blueprint/Character/Animation/AnimAssets/Stand/Equip/Thorwable/Equip_throwable_F_BaseBody_01_Rifle_Combat_Stand_Throw_Unequip_Static_Montage.Equip_throwable_F_BaseBody_01_Rifle_Combat_Stand_Throw_Unequip_Static_Montage") (struct :`GameplayTags` (struct :`(TagName` "Player.Event.Action.Equip"))) -2.0 "Equip"
          (:`OnCompleted`
            (`self.K2_EndAbility` :!label _label_2))
          (:`OnBlendOut`
            (goto _label_2))
          (:`OnInterrupted`
            (goto _label_2))
          (:`OnCancelled`
            (goto _label_2))
          (:`EventReceived`
            (`self.Attach_BackToHand_Weapon` "item_rSocket" _returnvalue_2)
            (`self.EquipWeaponHandle` _returnvalue_2)))))
    (else
      (`self.K2_EndAbility`))))

(fn `EquipWeaponHandle`
  (params (InputObject :type "Weapon_Base Object Reference"))
  (bind (_weaponanimlayertolink _equipanimmontage _weapontag _weaponinputmappingcontext _weaponabilities) (break `PlayerWeaponData` (`Weapon_Base.PlayerWeaponData` InputObject)))
  (`/Engine/EditorBlueprintResources/StandardMacros.IsValid` InputObject
    (:`Is Valid`
      (`|ExecutionSequence`
        (:`then_0`
          (`PlayerCharacter.Server_SetAnimLayer` (`self.GetPlayerCharacterFromActorInfo`) _weaponanimlayertolink))
        (:`then_1`
          (`self.IsLocallyControlled`
            (:`True`
              (`EnhancedInputSubsystemInterface.AddMappingContext` (pcsubsystem `EnhancedInputLocalPlayerSubsystem` (`self.GetPlayerControllerFromActorInfo`)) _weaponinputmappingcontext 1 (struct)))))
        (:`then_2`
          (`self.SetWeaponAbility` _weaponabilities InputObject))
        (:`then_3`
          (`BaseFunctionLibrary.AddGameplayTagToActor` (`self.GetPlayerCharacterFromActorInfo`) _weapontag true))))
    (:`Is Not Valid`
      (`KismetSystemLibrary.PrintString` "No value"))))

(fn `UnEquipWeaponHandle`
  (params (InputObject :type "Weapon_Base Object Reference"))
  (bind (_weaponanimlayertolink _equipanimmontage _weapontag _weaponinputmappingcontext) (break `PlayerWeaponData` (`Weapon_Base.PlayerWeaponData` InputObject)))
  (`/Engine/EditorBlueprintResources/StandardMacros.IsValid` InputObject
    (:`Is Valid`
      (`|ExecutionSequence`
        (:`then_0`
          (`PlayerCharacter.Server_SetAnimLayer` (`self.GetPlayerCharacterFromActorInfo`) null))
        (:`then_1`
          (`self.IsLocallyControlled`
            (:`True`
              (`EnhancedInputSubsystemInterface.RemoveMappingContext` (pcsubsystem `EnhancedInputLocalPlayerSubsystem` (`self.GetPlayerControllerFromActorInfo`)) _weaponinputmappingcontext (struct)))))
        (:`then_2`
          (`self.RemoveWeaponAbility` InputObject))
        (:`then_3`
          (`BaseFunctionLibrary.RemoveGameplayTagFromActor` (`self.GetPlayerCharacterFromActorInfo`) _weapontag true))))
    (:`Is Not Valid`
      (`KismetSystemLibrary.PrintString` "No value"))))