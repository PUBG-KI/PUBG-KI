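; Test gameplay ability that toggles between equipping and holstering the player's rifle, based on whether InventoryComponent has a current weapon.
; Equipping spawns and attaches a new BP_AK_47 and plays the slot montage in reverse; holstering plays it forward and reattaches the weapon to the primary slot.
; Gameplay events time the inventory update and helpers that add or remove the weapon's anim layers, input mapping and granted abilities.
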(event `self.K2_ActivateAbility`
  (bind _returnvalue (`self.GetOwningComponentFromActorInfo`))
  (bind _inventorycomponent (`PlayerCharacter.InventoryComponent` (`self.GetPlayerCharacterFromActorInfo`)))
  (bind _returnvalue_2 (`InventoryComponent.GetCurrentWeapon` _inventorycomponent))
  (`self.SetCanBeCanceled` false)
  (if (`KismetSystemLibrary.IsValid` (`InventoryComponent.GetCurrentWeapon` (`PlayerCharacter.InventoryComponent` (`self.GetPlayerCharacterFromActorInfo`))))
    (`AbilityTask_PlayMontageAndWait.CreatePlayMontageAndWaitProxy` "None" "/Game/Blueprint/Character/Animation/AnimAssets/Stand/Equip/Frimary/Rifle_Combat_Stand_PrimarySlot_Static_Montage.Rifle_Combat_Stand_PrimarySlot_Static_Montage" 2.0
      (:`then`
        (`AbilityTask_WaitGameplayEvent.WaitGameplayEvent` (struct :`TagName` "Player.Event.Action.UnEquip") null
          (:`EventReceived`
            (`self.UnEquipWeaponHandle` _returnvalue_2)
            (`KismetSystemLibrary.PrintString` "dddddddddddd")
            (`SceneComponent.K2_AttachToComponent` (`Actor.RootComponent` _returnvalue_2) (`self.GetOwningComponentFromActorInfo`) "slot_primarySocket" "SnapToTarget" "SnapToTarget" "KeepRelative" true)
            (`InventoryComponent.SetCurrentWeapon` _inventorycomponent null)
            (`self.K2_EndAbility`)))))
    (else
      (bind _returnvalue_3 (`|SpawnActorFromClass` "/Game/Blueprint/Weapon/BP_AK_47.BP_AK_47_C" (`SkinnedMeshComponent.GetBoneTransform` _returnvalue "ik_hand_gunSocket" "RTS_World") "Undefined" "MultiplyWithRoot" null null))
      (`SceneComponent.K2_AttachToComponent` (`Actor.RootComponent` _returnvalue_3) _returnvalue "item_rSocket" "SnapToTarget" "SnapToTarget" "KeepRelative" true)
      (`AbilityTask_PlayMontageAndWait.CreatePlayMontageAndWaitProxy` "None" "/Game/Blueprint/Character/Animation/AnimAssets/Stand/Equip/Frimary/Rifle_Combat_Stand_PrimarySlot_Static_Montage.Rifle_Combat_Stand_PrimarySlot_Static_Montage" -2.0 "None" true 1.0 1.7
        (:`then`
          (`AbilityTask_WaitGameplayEvent.WaitGameplayEvent` (struct :`TagName` "Player.Event.Action.Equip") null
            (:`EventReceived`
              (`InventoryComponent.SetCurrentWeapon` (`PlayerCharacter.InventoryComponent` (`self.GetPlayerCharacterFromActorInfo`)) _returnvalue_3)
              (`self.EquipWeaponHandle` (`InventoryComponent.GetCurrentWeapon` (`PlayerCharacter.InventoryComponent` (`self.GetPlayerCharacterFromActorInfo`))))
              (`self.K2_EndAbility`))))))))

(fn `EquipWeaponHandle`
  (params (self5 :type "Weapon_Base Object Reference"))
  (bind (_weaponanimlayertolink _equipanimmontage _weaponinputmappingcontext _weaponabilities) (break `PlayerWeaponData` (`Weapon_Base.WeaponData` self5)))
  (`/Engine/EditorBlueprintResources/StandardMacros.IsValid` self5
    (:`Is Valid`
      (`|ExecutionSequence`
        (:`then_0`
          (`SkeletalMeshComponent.LinkAnimClassLayers` (`self.GetOwningComponentFromActorInfo`) _weaponanimlayertolink))
        (:`then_1`
          (`EnhancedInputSubsystemInterface.AddMappingContext` (pcsubsystem `EnhancedInputLocalPlayerSubsystem` (`self.GetPlayerControllerFromActorInfo`)) _weaponinputmappingcontext 1 (struct)))
        (:`then_2`
          (bind _outgrantedabilityspechandles (`BaseAbilitySystemComponent.GrantPlayerWeaponAbilities` (`self.GetBaseAbilitySystemComponentFromActorInfo`) _weaponabilities (`self.GetAbilityLevel`)))
          (`Weapon_Base.AssignGrantedAbilitySpecHandles` self5 _outgrantedabilityspechandles))))
    (:`Is Not Valid`
      (`KismetSystemLibrary.PrintString` "No value"))))

(fn `UnEquipWeaponHandle`
  (params (Weapon :type "Weapon_Base Object Reference"))
  (bind (_weaponanimlayertolink _equipanimmontage _weaponinputmappingcontext) (break `PlayerWeaponData` (`Weapon_Base.WeaponData` Weapon)))
  (`/Engine/EditorBlueprintResources/StandardMacros.IsValid` Weapon
    (:`Is Valid`
      (`|ExecutionSequence`
        (:`then_0`
          (`SkeletalMeshComponent.UnlinkAnimClassLayers` (`self.GetOwningComponentFromActorInfo`) _weaponanimlayertolink))
        (:`then_1`
          (`EnhancedInputSubsystemInterface.RemoveMappingContext` (pcsubsystem `EnhancedInputLocalPlayerSubsystem` (`self.GetPlayerControllerFromActorInfo`)) _weaponinputmappingcontext (struct)))
        (:`then_2`
          (`BaseAbilitySystemComponent.RemoveGrantedPlayerWeaponAbilities` (`self.GetBaseAbilitySystemComponentFromActorInfo`) (`Weapon_Base.GetGrantedAbilitySpecHandles` Weapon)))))
    (:`Is Not Valid`
      (`KismetSystemLibrary.PrintString` "No value"))))