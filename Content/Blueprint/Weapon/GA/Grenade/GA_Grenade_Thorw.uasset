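; Gameplay ability for the grenade throw, driving the player's ready and release animations.
; Activation plays a prone or standing start montage and immediately adds the replicated Player.State.ThrowsReady tag.
; Ending plays the matching high-throw end montage, set to outlast the ability, and immediately removes the tag.
; The throw event tag is passed to that montage task but has no handler, and no grenade spawns here.
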(event `self.K2_ActivateAbility`
  (`KismetSystemLibrary.PrintString` "Hello" true true (struct :`G` 1.0 :`B` 0.021893 :`A` 1.0))
  (`PlayMontageAndWaitForEvent.PlayMontageAndWaitForEvent` "None" (`self.selectCurrentMontage_isProne_Throw` "/Game/Blueprint/Character/Animation/AnimAssets/Weapon/Grenade/Throw/ThrowPose_F_BaseBody_01_Grenade_Combat_Prone_Start_Montage.ThrowPose_F_BaseBody_01_Grenade_Combat_Prone_Start_Montage" "/Game/Blueprint/Character/Animation/AnimAssets/Weapon/Grenade/Throw/ThrowPose_F_BaseBody_01_Grenade_Combat_Stand_Start_Montage.ThrowPose_F_BaseBody_01_Grenade_Combat_Stand_Start_Montage") (struct) 2.0
    (:`then`
      (`BaseFunctionLibrary.AddGameplayTagToActor` (`self.GetPlayerCharacterFromActorInfo`) (struct :`TagName` "Player.State.ThrowsReady") true))))

(event `self.K2_OnEndAbility`
  (params (bWasCancelled :type Boolean))
  (`KismetSystemLibrary.PrintString` "ssssss" true true (struct :`R` 0.267227 :`B` 1.0 :`A` 1.0))
  (`PlayMontageAndWaitForEvent.PlayMontageAndWaitForEvent` "None" (`self.selectCurrentMontage_isProne_Throw` "/Game/Blueprint/Character/Animation/AnimAssets/Weapon/Grenade/Throw/ThrowPose_F_BaseBody_01_Grenade_Combat_Prone_High_End_Montage.ThrowPose_F_BaseBody_01_Grenade_Combat_Prone_High_End_Montage" "/Game/Blueprint/Character/Animation/AnimAssets/Weapon/Grenade/Throw/ThrowPose_F_BaseBody_01_Grenade_Combat_Stand_High_End_Montage.ThrowPose_F_BaseBody_01_Grenade_Combat_Stand_High_End_Montage") (struct :`GameplayTags` (struct :`(TagName` "Player.Event.Action.Throw"))) 2.0 "None" false
    (:`then`
      (`BaseFunctionLibrary.RemoveGameplayTagFromActor` (`self.GetPlayerCharacterFromActorInfo`) (struct :`TagName` "Player.State.ThrowsReady") true))))