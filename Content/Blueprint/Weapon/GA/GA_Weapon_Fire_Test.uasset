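; Test gameplay ability that fires the player's current gun, branching on its fire mode.
; Single plays montages, spawns one projectile and ends on montage completion; Auto starts a looping timer, which nothing here clears.
; SpawnProjectile decrements ammo and spawns BP_Test_Projectile at the muzzle socket with ballistics from the weapon data asset.
; Ammo checks with tag-activated fallback (apparently auto-reload) and the three-round burst starter are disconnected.
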(event `self.K2_ActivateAbilityFromEvent`
  (params (EventData :type "GameplayEventData Structure (by ref)"))
  ;[1 1 1] Comment
)

(event `Auto_fire`
  ;[1 1 1] 연발
  (`self.SpawnProjectile`))

(event `self.K2_ActivateAbility`
  (switch `EFiremodes` (`Gun_Base.GetFireMode` (`InventoryComponent.GetCurrentWeapon_GunBase` (`PlayerCharacter.InventoryComponent` (`self.GetPlayerCharacterFromActorInfo`))))
    (:`Auto`
      ;[1 1 1] 연발
      (`self.SpawnProjectile`)
      (`|PlayMontage` (`self.GetOwningComponentFromActorInfo`)
        (:`then`
          (bind _returnvalue (`KismetSystemLibrary.K2_SetTimerDelegate` (delegate `Auto_fire`) 0.1 true))
          (set `self.AutoHandle` _returnvalue))))
    (:`Single`
      ;[1 1 1] 단발
      (`|ExecutionSequence`
        (:`then_0`
          (`|PlayMontage` (`self.GetOwningComponentFromActorInfo`)))
        (:`then_1`
          (`self.SpawnProjectile`))
        (:`then_2`
          (`|PlayMontage` null "/Game/Blueprint/Weapon/Anim/AM_AK_47_Fire.AM_AK_47_Fire"
            (:`OnCompleted`
              (`self.K2_EndAbility`))))))))

(event `self.K2_OnEndAbility`
  (params (bWasCancelled :type Boolean))
  ;[1 1 1] 자동 재장전
)

(event `Semi_Auto`
  ;[1 1 1] 3점사
  (bind _counter (`/Engine/EditorBlueprintResources/StandardMacros.Do N` 2 :!label _label)
    (:`Exit`
      (if (> (`Gun_Base.GetBulletArmo` (`InventoryComponent.GetCurrentWeapon_GunBase` (`PlayerCharacter.InventoryComponent` (`self.GetPlayerCharacterFromActorInfo`)))) 0.0)
        (`self.SpawnProjectile`)
        (if (== _counter 2)
          (`KismetSystemLibrary.K2_ClearAndInvalidateTimerHandle` (`self.SemiHandle`))
          (`|ExecutionSequence`
            (:`then_0`
              (`KismetSystemLibrary.Delay` 0.3)
              (`self.K2_EndAbility`))
            (:`then_1`
              (goto _label :!via `Reset`)))
          (else
            (`KismetSystemLibrary.PrintString` "Single")))
        (else
          (`KismetSystemLibrary.K2_ClearAndInvalidateTimerHandle` (`self.SemiHandle`))
          (goto _label :!via `Reset`))))))

(fn `SpawnProjectile`
  (bind _inventorycomponent (`PlayerCharacter.InventoryComponent` (`self.GetPlayerCharacterFromActorInfo`)))
  (bind _returnvalue (`InventoryComponent.GetCurrentWeapon_GunBase` _inventorycomponent))
  (bind (_type _gunname _bullettype _gun_damage _armo _bullet_speed _bullet_crosssection _bullet_mass _bullet_dragcoefficiency) (break `WeaponData` (`Weapon_Base.GetWeaponDataAsset` (`InventoryComponent.GetCurrentWeapon` _inventorycomponent))))
  (bind _result (`/Engine/EditorBlueprintResources/StandardMacros.DecrementFloat` (`Gun_Base.GetBulletArmo` _returnvalue))
    (:`  `
      (`Gun_Base.SetBulletArom` _returnvalue _result)
      (`|SpawnActorFromClass` "/Game/Blueprint/Weapon/Projectile/BP_Test_Projectile.BP_Test_Projectile_C" (`SceneComponent.GetSocketTransform` (`Weapon_Base.WeaponSkeletalMeshComponent` _returnvalue) "ProjectileSocket" "RTS_World") "Undefined" "MultiplyWithRoot" null _gun_damage _bullet_speed _bullet_mass _bullet_crosssection _bullet_dragcoefficiency (`self.GetPlayerCharacterFromActorInfo`) (0.0 0.0 0.0) null null)
      (return))))